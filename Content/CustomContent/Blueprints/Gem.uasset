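; Gem actor with a mesh and point light that can be switched between Clear, Blue, Red and Green looks.
; Its SetColour event matches the colour to a gem material, light colour and intensity, then applies them to GemMesh and PointLight.
; Clear uses an uncoloured material with a dim white light, while the coloured variants glow much brighter in their matching hue.
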(event Custom|SetColour
  (params (Colour :type GemColours%20Enum :default "NewEnumerator0"))
  (switch Utilities|FlowControl|Switch|SwitchonGemColours Colour
    (:NewEnumerator0
      (Variables|Default|SetGemMaterial "/Game/CustomContent/Materials/Gem/MI_UncolouredGem.MI_UncolouredGem")
      (Variables|Default|SetLightColour (Utilities|Struct|MakeLinearColor 1.0 1.0 1.0 1.0))
      (Variables|Default|SetLightIntensity 0.25))
    (:NewEnumerator1
      (Variables|Default|SetGemMaterial "/Game/CustomContent/Materials/Gem/MI_BlueGem.MI_BlueGem")
      (Variables|Default|SetLightColour (Utilities|Struct|MakeLinearColor 0.0 0.0 1.0 1.0))
      (Variables|Default|SetLightIntensity 5.0))
    (:NewEnumerator2
      (Variables|Default|SetGemMaterial "/Game/CustomContent/Materials/Gem/MI_RedGem.MI_RedGem")
      (Variables|Default|SetLightColour (Utilities|Struct|MakeLinearColor 1.0 0.0 0.0 1.0))
      (Variables|Default|SetLightIntensity 5.0))
    (:NewEnumerator3
      (Variables|Default|SetGemMaterial "/Game/CustomContent/Materials/Gem/MI_GreenGem.MI_GreenGem")
      (Variables|Default|SetLightColour (Utilities|Struct|MakeLinearColor 0.0 1.0 0.0 1.0))
      (Variables|Default|SetLightIntensity 5.0)))
  (Rendering|Material|SetMaterial (Variables|Default|GetGemMesh) 0 (Variables|Default|GetGemMaterial))
  (Rendering|Components|Light|SetLightColor (Variables|Default|GetPointLight) (Variables|Default|GetLightColour) true)
  (Rendering|Components|Light|SetIntensity (Variables|Default|GetPointLight) (Variables|Default|GetLightIntensity)))

(event EventBeginPlay)

(event Collision|EventActorBeginOverlap
  (params (OtherActor :type Actor%20Object%20Reference)))

(event EventTick
  (params (DeltaSeconds :type Float%20%28single-precision%29)))

(fn ConstructionScript)