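; Balance scale puzzle actor that tilts a beam by weight and sets the torch state on its parent BP_BasePuzzle.
; Each tick it pins both pans' height to beam points and sums grounded Weight actors overlapping each side.
; The adjusted weight ratio sets the target tilt, and changes play a timeline that lerps beam pitch within clamped limits.
; When it finishes, the torch is on only if the beam is level and the right side holds objects.
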(event Custom|RotateBeam
  (bind _balancebeam (Variables|Default|GetBalanceBeam))
  (bind _maxtiltangle (Variables|Default|GetMaxTiltAngle))
  (bind _returnvalue (Transformation|GetWorldRotation _balancebeam))
  (bind (_roll _pitch _yaw) (Math|Rotator|BreakRotator _returnvalue))
  (Variables|Default|SetTiltValue (Math|Float|Clamp(Float) (Variables|Default|GetTiltValue) (* _maxtiltangle -1.0) _maxtiltangle))
  (bind _output_get (Variables|Default|SetStartTiltValue _pitch))
  (bind _tilttime (Timeline|BeamTime PlayFromStart)
    (:Update
      (Transformation|SetWorldRotation (Variables|Default|GetBalanceBeam) (Math|Rotator|MakeRotator _roll (Math|Float|Lerp _output_get (Variables|Default|GetTiltValue) _tilttime) _yaw) false false))
    (:Finished
      (bind _asbp_base_puzzle (Utilities|Casting|CastToBP_BasePuzzle (Actor|GetAttachParentActor)))
      (Default|SetTorchState _asbp_base_puzzle (and (== (Variables|Default|GetTiltValue) 0.0) (> (Variables|Default|GetObjectNum) 0))))))

(event EventBeginPlay
  (Variables|Default|SetHeightOffset (- (.Z (Math|Vector|BreakVector (Transformation|GetWorldLocation (Variables|Default|GetRSide)))) (.Z (Math|Vector|BreakVector (Transformation|GetWorldLocation (Variables|Default|GetRSidePoint)))))))

(event Collision|EventActorBeginOverlap
  (params (OtherActor :type Actor%20Object%20Reference)))

(event EventTick
  (params (DeltaSeconds :type Float%20%28single-precision%29))
  (bind _lside (Variables|Default|GetLside))
  (bind _rsidecoll (Variables|Default|GetRSideColl))
  (bind _rside (Variables|Default|GetRSide))
  (bind _overlappingactors (Collision|GetOverlappingActors _rsidecoll "/Game/CustomContent/Blueprints/Weight.Weight_C" :!class /Script/Engine.PrimitiveComponent))
  (Utilities|FlowControl|Sequence
    (:then_0
      (bind _outputvector (CallFunction|UpdateScaleHeight (Transformation|GetWorldLocation _rside) (Variables|Default|GetHeightOffset) (Transformation|GetWorldLocation (Variables|Default|GetRSidePoint))))
      (Transformation|SetWorldLocation _rside _outputvector false false)
      (bind _outputvector_2 (CallFunction|UpdateScaleHeight (Transformation|GetWorldLocation _lside) (Variables|Default|GetHeightOffset) (Transformation|GetWorldLocation (Variables|Default|GetLSidePoint))))
      (Transformation|SetWorldLocation _lside _outputvector_2 false false))
    (:then_1
      (Variables|Default|SetLWeight 0.0)
      (for _array_element (Collision|GetOverlappingActors (Variables|Default|GetLSideColl) "/Game/CustomContent/Blueprints/Weight.Weight_C" :!class /Script/Engine.PrimitiveComponent)
        (bind _asweight (Utilities|Casting|CastToWeight _array_element))
        (if (Variables|/Game/CustomContent/Blueprints/Weight.Weight_C|GetIsGrounded _asweight)
          (Variables|Default|SetLWeight (+ (Variables|/Game/CustomContent/Blueprints/Weight.Weight_C|GetWeight _asweight) (Variables|Default|GetLWeight))))))
    (:then_2
      (Variables|Default|SetRWeight 0.0)
      (Variables|Default|SetObjectNum (Utilities|Array|Length _overlappingactors))
      (for _array_element_2 _overlappingactors
        (bind _asweight_2 (Utilities|Casting|CastToWeight _array_element_2))
        (if (Variables|/Game/CustomContent/Blueprints/Weight.Weight_C|GetIsGrounded _asweight_2)
          (Variables|Default|SetRWeight (+ (Variables|/Game/CustomContent/Blueprints/Weight.Weight_C|GetWeight _asweight_2) (Variables|Default|GetRWeight))))))
    (:then_3
      (CallFunction|AdjustBeamRotation))))

(fn ConstructionScript)

(fn UpdateScaleHeight
  (params (InputScaleTrans :type Vector) (Height :type Float%20%28double-precision%29) (InputBeamTrans :type Vector))
  (bind (_x _y) (Math|Vector|BreakVector InputScaleTrans))
  (return (Math|Vector|MakeVector _x _y (+ Height (.Z (Math|Vector|BreakVector InputBeamTrans))))))

(fn AdjustBeamRotation
  (Variables|Default|SetPrevTiltValue (Variables|Default|GetTiltValue))
  (if (and (== (Utilities|AdjustedLWeight) 0.0) (!= (Utilities|AdjustedRWeight) 0.0))
    (Variables|Default|SetTiltValue (Variables|Default|GetMaxTiltAngle))
    (if (!= (Variables|Default|GetPrevTiltValue) (Variables|Default|GetTiltValue)) :!label _label
      (CallFunction|RotateBeam))
    (elif (and (== (Utilities|AdjustedRWeight) 0.0) (!= (Utilities|AdjustedLWeight) 0.0))
      (Variables|Default|SetTiltValue (* (Variables|Default|GetMaxTiltAngle) -1.0))
      (goto _label)
      (elif (== (Utilities|AdjustedRWeight) (Utilities|AdjustedLWeight))
        (Variables|Default|SetTiltValue 0.0)
        (goto _label)
        (elif (> (Utilities|AdjustedRWeight) (Utilities|AdjustedLWeight))
          (Variables|Default|SetTiltValue (* (/ (Utilities|AdjustedRWeight) (Utilities|AdjustedLWeight)) (/ (Variables|Default|GetMaxTiltAngle) 2.0)))
          (goto _label)
          (elif (> (Utilities|AdjustedLWeight) (Utilities|AdjustedRWeight))
            (Variables|Default|SetTiltValue (* (/ (Utilities|AdjustedLWeight) (Utilities|AdjustedRWeight)) (/ (Variables|Default|GetMaxTiltAngle) -2.0)))
            (goto _label)))))))