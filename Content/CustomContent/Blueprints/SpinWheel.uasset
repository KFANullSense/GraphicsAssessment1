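; Two-wheel number puzzle that lights or clears a torch on its parent BasePuzzle actor when the dialed two-digit value matches a target.
; BeginPlay derives the target from four random values as (A+B)*(C-D).
; Each increment event advances its digit with wraparound and plays a timeline rotating that wheel, ignoring input while it spins.
; Timeline updates compare the combined digits to the target and pass the result to SetTorchState.
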(event Custom|IncrementLeftWheel
  (bind _wheell (Variables|Default|GetWheelL))
  (if (not (Variables|Default|GetLRotating))
    (bind _output (CallFunction|IncrementNum (Variables|Default|GetLeftWheelVal)))
    (Variables|Default|SetLeftWheelVal _output)
    (Variables|Default|SetLRotating true)
    (Variables|Default|SetStartLRot (Variables|/Script/Engine.SceneComponent|GetRelativeRotation _wheell))
    (bind _timepassed (Timeline|LWheelTimeline PlayFromStart)
      (:Update
        (Transformation|SetRelativeRotation _wheell (Math|Rotator|CombineRotators (Variables|Default|GetStartLRot) (Math|Rotator|MakeRotator (* _timepassed -36.0) 0.0 0.0)) false false)
        (bind _result (CallFunction|ValidateWheelNum))
        (bind _asbase_puzzle (Utilities|Casting|CastToBasePuzzle (Actor|GetAttachParentActor)))
        (Default|SetTorchState _asbase_puzzle _result))
      (:Finished
        (Variables|Default|SetLRotating false)))))

(event Custom|IncrementRightWheel
  (bind _wheelr (Variables|Default|GetWheelR))
  (if (not (Variables|Default|GetRRotating))
    (bind _output (CallFunction|IncrementNum (Variables|Default|GetRightWheelVal)))
    (Variables|Default|SetRightWheelVal _output)
    (Variables|Default|SetRRotating true)
    (Variables|Default|SetStartRRot (Variables|/Script/Engine.SceneComponent|GetRelativeRotation _wheelr))
    (bind _timepassed (Timeline|RWheelTimeline PlayFromStart)
      (:Update
        (Transformation|SetRelativeRotation _wheelr (Math|Rotator|CombineRotators (Variables|Default|GetStartRRot) (Math|Rotator|MakeRotator (* _timepassed -36.0) 0.0 0.0)) false false)
        (bind _result (CallFunction|ValidateWheelNum))
        (bind _asbase_puzzle (Utilities|Casting|CastToBasePuzzle (Actor|GetAttachParentActor)))
        (Default|SetTorchState _asbase_puzzle _result))
      (:Finished
        (Variables|Default|SetRRotating false)))))

(event EventBeginPlay
  (bind _output_get (Variables|Default|SetdVar (Math|Random|RandomIntegerinRange 1 9)))
  (Variables|Default|SetcVar (Math|Integer|Clamp(Integer) (Math|Random|RandomIntegerinRange _output_get (+ _output_get 5)) 1 10))
  (Variables|Default|SetbVar (Math|Random|RandomIntegerinRange 1 9))
  (Variables|Default|SetaVar (Math|Random|RandomIntegerinRange 1 9))
  (Variables|Default|SetTargetNumber (* (+ (Variables|Default|GetaVar) (Variables|Default|GetbVar)) (- (Variables|Default|GetcVar) (Variables|Default|GetdVar)))))

(fn ConstructionScript)

(fn CalculateWheelVal
  (return (+ (* (Variables|Default|GetLeftWheelVal) 10) (Variables|Default|GetRightWheelVal))))

(fn ValidateWheelNum
  (bind _finalnum (CallFunction|CalculateWheelVal))
  (return (== _finalnum (Variables|Default|GetTargetNumber))))

(fn IncrementNum
  (params (Input :type Integer))
  (bind _returnvalue (+ Input 1))
  (if (>= _returnvalue 10)
    (return (- _returnvalue 10))
    (else
      (return _returnvalue))))