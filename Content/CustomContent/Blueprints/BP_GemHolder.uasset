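; BP_GemHolder is a gem-sorting puzzle piece with a pedestal that reveals a gem's colour and containers for red and blue gems.
; Container overlaps count correctly typed gems against required totals, and removal from the pedestal or matching container clears colour.
; Each count change recolours contained gems green or colourless and sets the parent BP_BasePuzzle's torch state.
; The blue recolour loop is nested inside the red one.
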(event OnComponentBeginOverlap(PedestalColl)
  (params (OverlappedComponent :type Primitive%20Component%20Object%20Reference) (OtherActor :type Actor%20Object%20Reference) (OtherComp :type Primitive%20Component%20Object%20Reference) (OtherBodyIndex :type Integer) (bFromSweep :type Boolean) (SweepResult :type Hit%20Result%20Structure%20%28by%20ref%29))
  ;[0.15 0.15 0.15 0.5] When gem placed on pedestal, reveal its colour
  (bind _asbp_gem (Utilities|Casting|CastToBP_Gem OtherActor))
  (Default|SetColour _asbp_gem (Variables|/Game/CustomContent/Blueprints/BP_Gem.BP_Gem_C|GetGemType _asbp_gem)))

(event OnComponentEndOverlap(PedestalColl)
  (params (OverlappedComponent :type Primitive%20Component%20Object%20Reference) (OtherActor :type Actor%20Object%20Reference) (OtherComp :type Primitive%20Component%20Object%20Reference) (OtherBodyIndex :type Integer))
  ;[0.15 0.15 0.15 0.5] When gem removed from pedestal, clear colour
  (bind _asbp_gem (Utilities|Casting|CastToBP_Gem OtherActor))
  (Default|SetColour _asbp_gem "NewEnumerator0"))

(event OnComponentBeginOverlap(BlueColl)
  (params (OverlappedComponent :type Primitive%20Component%20Object%20Reference) (OtherActor :type Actor%20Object%20Reference) (OtherComp :type Primitive%20Component%20Object%20Reference) (OtherBodyIndex :type Integer) (bFromSweep :type Boolean) (SweepResult :type Hit%20Result%20Structure%20%28by%20ref%29))
  ;[0.15 0.15 0.15 0.5] If blue gem placed in blue container, add one to blue gem num
  (bind _result (CallFunction|CheckGemType OtherActor "NewEnumerator1"))
  (if _result
    (Variables|Default|SetcurrentBlueGems (+ 1 (Variables|Default|GetcurrentBlueGems)))
    ;[0.15 0.15 0.15 0.5] If all gems in right place, set all gem colours to green, otherwise set to colourless
    (if (and (>= (Variables|Default|GetcurrentBlueGems) (Variables|Default|GetRequiredBlueGems)) (>= (Variables|Default|GetcurrentRedGems) (Variables|Default|GetRequiredRedGems)))
      (CallFunction|SetCurrentGemColours "NewEnumerator3")
      (CallFunction|SetParentTorchState true)
      (else
        (CallFunction|SetCurrentGemColours "NewEnumerator0")
        (CallFunction|SetParentTorchState false)))))

(event OnComponentEndOverlap(BlueColl)
  (params (OverlappedComponent :type Primitive%20Component%20Object%20Reference) (OtherActor :type Actor%20Object%20Reference) (OtherComp :type Primitive%20Component%20Object%20Reference) (OtherBodyIndex :type Integer))
  ;[0.15 0.15 0.15 0.5] If blue gem removed from blue container, remove one from blue gem num
  (bind _result (CallFunction|CheckGemType OtherActor "NewEnumerator1"))
  (if _result
    (bind _asbp_gem (Utilities|Casting|CastToBP_Gem OtherActor))
    (Default|SetColour _asbp_gem "NewEnumerator0")
    (Variables|Default|SetcurrentBlueGems (- (Variables|Default|GetcurrentBlueGems) 1))
    ;[0.15 0.15 0.15 0.5] If all gems in right place, set all gem colours to green, otherwise set to colourless
    (if (and (>= (Variables|Default|GetcurrentBlueGems) (Variables|Default|GetRequiredBlueGems)) (>= (Variables|Default|GetcurrentRedGems) (Variables|Default|GetRequiredRedGems)))
      (CallFunction|SetCurrentGemColours "NewEnumerator3")
      (CallFunction|SetParentTorchState true)
      (else
        (CallFunction|SetCurrentGemColours "NewEnumerator0")
        (CallFunction|SetParentTorchState false)))))

(event OnComponentBeginOverlap(RedColl)
  (params (OverlappedComponent :type Primitive%20Component%20Object%20Reference) (OtherActor :type Actor%20Object%20Reference) (OtherComp :type Primitive%20Component%20Object%20Reference) (OtherBodyIndex :type Integer) (bFromSweep :type Boolean) (SweepResult :type Hit%20Result%20Structure%20%28by%20ref%29))
  ;[0.15 0.15 0.15 0.5] If red gem placed in red container, add one to red gem num
  (bind _result (CallFunction|CheckGemType OtherActor "NewEnumerator2"))
  (if _result
    (Variables|Default|SetcurrentRedGems (+ 1 (Variables|Default|GetcurrentRedGems)))
    ;[0.15 0.15 0.15 0.5] If all gems in right place, set all gem colours to green, otherwise set to colourless
    (if (and (>= (Variables|Default|GetcurrentBlueGems) (Variables|Default|GetRequiredBlueGems)) (>= (Variables|Default|GetcurrentRedGems) (Variables|Default|GetRequiredRedGems)))
      (CallFunction|SetCurrentGemColours "NewEnumerator3")
      (CallFunction|SetParentTorchState true)
      (else
        (CallFunction|SetCurrentGemColours "NewEnumerator0")
        (CallFunction|SetParentTorchState false)))))

(event OnComponentEndOverlap(RedColl)
  (params (OverlappedComponent :type Primitive%20Component%20Object%20Reference) (OtherActor :type Actor%20Object%20Reference) (OtherComp :type Primitive%20Component%20Object%20Reference) (OtherBodyIndex :type Integer))
  ;[0.15 0.15 0.15 0.5] If red gem removed from red container, remove one from gem num
  (bind _result (CallFunction|CheckGemType OtherActor "NewEnumerator2"))
  (if _result
    (bind _asbp_gem (Utilities|Casting|CastToBP_Gem OtherActor))
    (Default|SetColour _asbp_gem "NewEnumerator0")
    (Variables|Default|SetcurrentRedGems (- (Variables|Default|GetcurrentRedGems) 1))
    ;[0.15 0.15 0.15 0.5] If all gems in right place, set all gem colours to green, otherwise set to colourless
    (if (and (>= (Variables|Default|GetcurrentBlueGems) (Variables|Default|GetRequiredBlueGems)) (>= (Variables|Default|GetcurrentRedGems) (Variables|Default|GetRequiredRedGems)))
      (CallFunction|SetCurrentGemColours "NewEnumerator3")
      (CallFunction|SetParentTorchState true)
      (else
        (CallFunction|SetCurrentGemColours "NewEnumerator0")
        (CallFunction|SetParentTorchState false)))))

(event EventBeginPlay)

(event Collision|EventActorBeginOverlap
  (params (OtherActor :type Actor%20Object%20Reference)))

(event EventTick
  (params (DeltaSeconds :type Float%20%28single-precision%29)))

(fn ConstructionScript)

(fn CheckGemType
  (params (Object :type Object%20Object%20Reference) (DesiredType :type E_GemColours%20Enum :default "NewEnumerator0"))
  (bind _asbp_gem (Utilities|Casting|CastToBP_Gem Object))
  (return (== (Variables|/Game/CustomContent/Blueprints/BP_Gem.BP_Gem_C|GetGemType _asbp_gem) (Math|Byte|MakeLiteralByte DesiredType))))

(fn SetCurrentGemColours
  (params (ColourToSet :type E_GemColours%20Enum :default "NewEnumerator0"))
  ;[0.15 0.15 0.15 0.5] Set colour of gems in containers
  (for _array_element (Collision|GetOverlappingActors (Variables|Default|GetRedColl) "/Game/CustomContent/Blueprints/BP_Gem.BP_Gem_C" :!class /Script/Engine.PrimitiveComponent)
    (bind _asbp_gem (Utilities|Casting|CastToBP_Gem _array_element))
    (Default|SetColour _asbp_gem ColourToSet)
    (for _array_element_2 (Collision|GetOverlappingActors (Variables|Default|GetBlueColl) "/Game/CustomContent/Blueprints/BP_Gem.BP_Gem_C" :!class /Script/Engine.PrimitiveComponent)
      (bind _asbp_gem_2 (Utilities|Casting|CastToBP_Gem _array_element_2))
      (Default|SetColour _asbp_gem_2 ColourToSet))))

(fn SetParentTorchState
  (params (Value :type Boolean))
  (bind _asbp_base_puzzle (Utilities|Casting|CastToBP_BasePuzzle (Actor|GetAttachParentActor)))
  (Default|SetTorchState _asbp_base_puzzle Value))