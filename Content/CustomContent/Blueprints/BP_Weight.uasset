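; BP_Weight is a weight actor built around a Cube component that tracks whether it is resting on a surface.
; Each Tick fires a Visibility line trace down from the cube's center, sized from half its Z scale plus a buffer, and stores the hit result in IsGrounded.
; BeginPlay caches the cube's starting relative yaw, though nothing in these graphs reads it.
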(event EventBeginPlay
  ;[0.15 0.15 0.15 0.5] On start, store Z rotation value
  (Variables|Default|SetStartingZRot (.Yaw (Math|Rotator|BreakRotator (Variables|/Script/Engine.SceneComponent|GetRelativeRotation (Variables|Default|GetCube)))))
  (|CallParentFunction))

(event Collision|EventActorBeginOverlap
  (params (OtherActor :type Actor%20Object%20Reference))
  (|CallParentFunction OtherActor) ; This node is disabled and will not be called.\nDrag off pins to build functionality.
)

(event EventTick
  (params (DeltaSeconds :type Float%20%28single-precision%29))
  (bind _cube (Variables|Default|GetCube))
  (bind _returnvalue (Transformation|GetWorldLocation _cube))
  ;[0.15 0.15 0.15 0.5] Every frame, check if weight is touching the ground
  ;;[0.15 0.15 0.15 0.5] Raycast downwards using calculated down vector
  (bind _returnvalue_2 (Collision|LineTraceByChannel _returnvalue (+ _returnvalue (* (* (Math|Vector|VectorUp) (Math|Float|MakeLiteralFloat -1.0)) (+ (/ (.Z (Math|Vector|BreakVector (Transformation|GetWorldScale (Variables|Default|GetCube)))) 2.0) 25.0))) "TraceTypeQuery1" false 0 "None"))
  (Variables|Default|SetIsGrounded _returnvalue_2)
  (|CallParentFunction DeltaSeconds))

(fn ConstructionScript
  (|CallParentFunction))