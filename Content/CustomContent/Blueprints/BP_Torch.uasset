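; BP_Torch is a torch actor that can be switched between lit and unlit, and it starts unlit on BeginPlay.
; The SetTorchState event swaps the second material slot of TorchModel between an on and an off material and shows or hides the PointLight to match.
; It records the result in IsTorchLit, and nothing in this Blueprint lights the torch itself.
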(event Custom|SetTorchState
  (params (TorchLit :type Boolean))
  (if TorchLit
    (Rendering|Material|SetMaterial (Variables|Default|GetTorchModel) 1 "/Game/CustomContent/Materials/Torch/MI_TorchOnInstance.MI_TorchOnInstance")
    (Rendering|SetVisibility (Variables|Default|GetPointLight) true false)
    (Variables|Default|SetIsTorchLit true)
    (else
      (Rendering|Material|SetMaterial (Variables|Default|GetTorchModel) 1 "/Game/CustomContent/Materials/Torch/M_TorchOff.M_TorchOff")
      (Rendering|SetVisibility (Variables|Default|GetPointLight) false false)
      (Variables|Default|SetIsTorchLit false))))

(event EventBeginPlay
  ;[0.15 0.15 0.15 0.5] At start of game, set all torches to off
  (CallFunction|SetTorchState false))

(event Collision|EventActorBeginOverlap
  (params (OtherActor :type Actor%20Object%20Reference)))

(event EventTick
  (params (DeltaSeconds :type Float%20%28single-precision%29)))

(fn ConstructionScript)