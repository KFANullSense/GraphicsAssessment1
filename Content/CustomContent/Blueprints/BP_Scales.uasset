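; Balance scale puzzle piece that tilts according to the BP_Weight actors placed on its two sides.
; Each tick keeps both sides level with their beam points, sums grounded overlapping weights per side and derives a clamped tilt from the weight ratio.
; Tilt changes play a timeline that rotates the beam.
; When it finishes, the parent BP_BasePuzzle's torch is lit only if the beam is balanced with weights present.
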(event Custom|RotateBeam
  (bind _balancebeam (Variables|Default|GetBalanceBeam))
  (bind _maxtiltangle (Variables|Default|GetMaxTiltAngle))
  (bind _returnvalue (Transformation|GetWorldRotation _balancebeam))
  (bind (_roll _pitch _yaw) (Math|Rotator|BreakRotator _returnvalue))
  (Variables|Default|SetTiltValue (Math|Float|Clamp(Float) (Variables|Default|GetTiltValue) (* _maxtiltangle -1.0) _maxtiltangle))
  ;[0.15 0.15 0.15 0.5] Rotate beam to target angle over time
  (bind _output_get (Variables|Default|SetStartTiltValue _pitch))
  (bind _tilttime (Timeline|BeamTime PlayFromStart)
    (:Update
      (Transformation|SetWorldRotation (Variables|Default|GetBalanceBeam) (Math|Rotator|MakeRotator _roll (Math|Float|Lerp _output_get (Variables|Default|GetTiltValue) _tilttime) _yaw) false false))
    (:Finished
      ;[0.15 0.15 0.15 0.5] If beam is balanced and there are weights on, set torch on, otherwise set off
      (bind _asbp_base_puzzle (Utilities|Casting|CastToBP_BasePuzzle (Actor|GetAttachParentActor)))
      (Default|SetTorchState _asbp_base_puzzle (and (== (Variables|Default|GetTiltValue) 0.0) (> (Variables|Default|GetObjectNum) 0))))))

(event EventBeginPlay
  ;[0.15 0.15 0.15 0.5] At start, set height offset (both sides of scale start in middle so either works for finding offset)
  (Variables|Default|SetHeightOffset (- (.Z (Math|Vector|BreakVector (Transformation|GetWorldLocation (Variables|Default|GetRSide)))) (.Z (Math|Vector|BreakVector (Transformation|GetWorldLocation (Variables|Default|GetRSidePoint)))))))

(event Collision|EventActorBeginOverlap
  (params (OtherActor :type Actor%20Object%20Reference)))

(event EventTick
  (params (DeltaSeconds :type Float%20%28single-precision%29))
  (bind _lside (Variables|Default|GetLside))
  (bind _rside (Variables|Default|GetRSide))
  (Utilities|FlowControl|Sequence ; Every tick, do these steps
    (:then_0
      ;[0.15 0.15 0.15 0.5] First, set heights of scale sides
      (bind _outputvector (CallFunction|UpdateScaleHeight (Transformation|GetWorldLocation _rside) (Variables|Default|GetHeightOffset) (Transformation|GetWorldLocation (Variables|Default|GetRSidePoint))))
      (Transformation|SetWorldLocation _rside _outputvector false false)
      (bind _outputvector_2 (CallFunction|UpdateScaleHeight (Transformation|GetWorldLocation _lside) (Variables|Default|GetHeightOffset) (Transformation|GetWorldLocation (Variables|Default|GetLSidePoint))))
      (Transformation|SetWorldLocation _lside _outputvector_2 false false))
    (:then_1
      ;[0.15 0.15 0.15 0.5] Next, find all weights that are placed on the left scale and store the sum of their weight values
      (Variables|Default|SetLWeight 0.0)
      (for _array_element (Collision|GetOverlappingActors (Variables|Default|GetLSideColl) "/Game/CustomContent/Blueprints/BP_Weight.BP_Weight_C" :!class /Script/Engine.PrimitiveComponent)
        (bind _asweight (Utilities|Casting|CastToBP_Weight _array_element))
        (if (Variables|/Game/CustomContent/Blueprints/BP_Weight.BP_Weight_C|GetIsGrounded _asweight)
          (Variables|Default|SetLWeight (+ (Variables|/Game/CustomContent/Blueprints/BP_Weight.BP_Weight_C|GetWeight _asweight) (Variables|Default|GetLWeight))))))
    (:then_2
      ;[0.15 0.15 0.15 0.5] Next, do the same for the right scale
      (Variables|Default|SetRWeight 0.0)
      (for _array_element_2 (Collision|GetOverlappingActors (Variables|Default|GetRSideColl) "/Game/CustomContent/Blueprints/BP_Weight.BP_Weight_C" :!class /Script/Engine.PrimitiveComponent)
        (bind _asweight_2 (Utilities|Casting|CastToBP_Weight _array_element_2))
        (if (Variables|/Game/CustomContent/Blueprints/BP_Weight.BP_Weight_C|GetIsGrounded _asweight_2)
          (Variables|Default|SetRWeight (+ (Variables|/Game/CustomContent/Blueprints/BP_Weight.BP_Weight_C|GetWeight _asweight_2) (Variables|Default|GetRWeight))))))
    (:then_3
      ;[0.15 0.15 0.15 0.5] Next, store number of weights on scales
      (Variables|Default|SetObjectNum (+ (Utilities|Array|Length (Collision|GetOverlappingActors (Variables|Default|GetLSideColl) "/Game/CustomContent/Blueprints/BP_Weight.BP_Weight_C" :!class /Script/Engine.PrimitiveComponent)) (Utilities|Array|Length (Collision|GetOverlappingActors (Variables|Default|GetRSideColl) "/Game/CustomContent/Blueprints/BP_Weight.BP_Weight_C" :!class /Script/Engine.PrimitiveComponent)))))
    (:then_4
      (CallFunction|AdjustBeamRotation) ; Finally, adjust beam rotation to tilt angle
    )))

(fn ConstructionScript)

(fn UpdateScaleHeight
  (params (InputScaleTrans :type Vector) (Height :type Float%20%28double-precision%29) (InputBeamTrans :type Vector))
  (bind (_x _y) (Math|Vector|BreakVector InputScaleTrans))
  (return (Math|Vector|MakeVector _x _y (+ Height (.Z (Math|Vector|BreakVector InputBeamTrans))))))

(fn AdjustBeamRotation
  (Variables|Default|SetPrevTiltValue (Variables|Default|GetTiltValue))
  ;[0.15 0.15 0.15 0.5] If right side has weight and left doesn't, fully tip right side
  (if (and (== (Utilities|AdjustedLWeight) 0.0) (!= (Utilities|AdjustedRWeight) 0.0))
    (Variables|Default|SetTiltValue (Variables|Default|GetMaxTiltAngle))
    ;[0.15 0.15 0.15 0.5] If value is different than last tick, rotate the beam
    (if (!= (Variables|Default|GetPrevTiltValue) (Variables|Default|GetTiltValue)) :!label _label
      (CallFunction|RotateBeam))
    (else
      ;[0.15 0.15 0.15 0.5] If left side has weight and right doesn't, fully tip left side
      (if (and (== (Utilities|AdjustedRWeight) 0.0) (!= (Utilities|AdjustedLWeight) 0.0))
        (Variables|Default|SetTiltValue (* (Variables|Default|GetMaxTiltAngle) -1.0))
        (goto _label)
        (else
          ;[0.15 0.15 0.15 0.5] If both sides are even, set tilt value to zero
          (if (== (Utilities|AdjustedRWeight) (Utilities|AdjustedLWeight))
            (Variables|Default|SetTiltValue 0.0)
            (goto _label)
            (else
              ;[0.15 0.15 0.15 0.5] If right weight is larger than left weight, calculate and tip towards right side
              (if (> (Utilities|AdjustedRWeight) (Utilities|AdjustedLWeight))
                (Variables|Default|SetTiltValue (* (/ (Utilities|AdjustedRWeight) (Utilities|AdjustedLWeight)) (/ (Variables|Default|GetMaxTiltAngle) 2.0)))
                (goto _label)
                (else
                  ;[0.15 0.15 0.15 0.5] If left weight is larger than right weight, calculate and tip towards left side
                  (if (> (Utilities|AdjustedLWeight) (Utilities|AdjustedRWeight))
                    (Variables|Default|SetTiltValue (* (/ (Utilities|AdjustedLWeight) (Utilities|AdjustedRWeight)) (/ (Variables|Default|GetMaxTiltAngle) -2.0)))
                    (goto _label)))))))))))