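; TreasureRoom is a room actor that gates a treasure door behind a torch puzzle and holds a treasure chest.
; On BeginPlay it caches every BP_Torch in the level.
; When the player enters the door trigger, the door child actor plays its open animation only if all torches are lit.
; Entering the treasure trigger opens the chest child actor once, independent of the torches.
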(event OnComponentBeginOverlap(DoorColl)
  (params (OverlappedComponent :type Primitive%20Component%20Object%20Reference) (OtherActor :type Actor%20Object%20Reference) (OtherComp :type Primitive%20Component%20Object%20Reference) (OtherBodyIndex :type Integer) (bFromSweep :type Boolean) (SweepResult :type Hit%20Result%20Structure%20%28by%20ref%29))
  (Utilities|Casting|CastToBP_CustomFPSCharacter OtherActor)
  (if (not (Variables|Default|GetIsDoorOpen))
    (Variables|Default|SetAllTorchesLit true)
    (bind _array_element (Utilities|Array|ForEachLoopwithBreak (Variables|Default|GetTorches) :!label _label)
      (:LoopBody
        (if (not (Variables|/Game/CustomContent/Blueprints/BP_Torch.BP_Torch_C|GetIsTorchLit _array_element))
          (Variables|Default|SetAllTorchesLit false)
          (goto _label Break)))
      (:Completed
        (if (Variables|Default|GetAllTorchesLit)
          (CallFunction|OpenDoor))))))

(event OnComponentBeginOverlap(TreasureColl)
  (params (OverlappedComponent :type Primitive%20Component%20Object%20Reference) (OtherActor :type Actor%20Object%20Reference) (OtherComp :type Primitive%20Component%20Object%20Reference) (OtherBodyIndex :type Integer) (bFromSweep :type Boolean) (SweepResult :type Hit%20Result%20Structure%20%28by%20ref%29))
  (Utilities|Casting|CastToBP_CustomFPSCharacter OtherActor)
  (if (not (Variables|Default|GetIsChestOpen))
    (Variables|Default|SetIsChestOpen true)
    (CallFunction|OpenChest)))

(event Custom|OpenDoor
  (Variables|Default|SetIsDoorOpen true)
  (bind _astreasure_door (Utilities|Casting|CastToTreasureDoor (Variables|/Script/Engine.ChildActorComponent|GetChildActor (Variables|Default|GetTreasureDoor))))
  (Default|OpenDoorAnimation _astreasure_door))

(event Custom|OpenChest
  (bind _astreasure_chest (Utilities|Casting|CastToTreasureChest (Variables|/Script/Engine.ChildActorComponent|GetChildActor (Variables|Default|GetTreasureChest))))
  (Default|OpenChestAnimation _astreasure_chest))

(event EventBeginPlay
  (bind _outactors (Actor|GetAllActorsOfClass "/Game/CustomContent/Blueprints/BP_Torch.BP_Torch_C"))
  (Variables|Default|SetTorches _outactors))

(event Collision|EventActorBeginOverlap
  (params (OtherActor :type Actor%20Object%20Reference)))

(fn ConstructionScript)