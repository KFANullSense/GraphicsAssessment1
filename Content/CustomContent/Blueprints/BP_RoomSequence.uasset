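; Room actor that runs a one-time lighting reveal when its trigger volume is overlapped, starting with torches and lights off.
; A timeline brightens an eye's dynamic material, then TurnOnLights steps through component groups one second apart, lighting child torches.
; TurnOnLights also restarts a shared LightTimeline meant to ramp the current group's point and rect light intensities.
; Three boxes lose collision once the first group's delay ends.
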(event OnComponentBeginOverlap(PlayerTrigger)
  (params (OverlappedComponent :type Primitive%20Component%20Object%20Reference) (OtherActor :type Actor%20Object%20Reference) (OtherComp :type Primitive%20Component%20Object%20Reference) (OtherBodyIndex :type Integer) (bFromSweep :type Boolean) (SweepResult :type Hit%20Result%20Structure%20%28by%20ref%29))
  (if (not (Variables|Default|GetHasTriggered))
    (Variables|Default|SetHasTriggered true)
    (bind _timefloat (Timeline|EyeTrigger PlayFromStart)
      (:Update
        (Rendering|Material|SetScalarParameterValue (Variables|Default|GetEyeMat) "LightIntensity" (* _timefloat 4.0) :!class /Script/Engine.MaterialInstanceDynamic))
      (:Finished
        (Variables|Default|SetMult 5e+03)
        (Utilities|TurnonLights (Variables|Default|GetFirstLights)
          (:Output
            (Utilities|FlowControl|Sequence
              (:then_0
                (Utilities|TurnonLights (Variables|Default|GetSecondLights)
                  (:Output
                    (Utilities|TurnonLights (Variables|Default|GetThirdLights)
                      (:Output
                        (Utilities|TurnonLights (Variables|Default|GetFourthLights)
                          (:Output
                            (Utilities|TurnonLights (Variables|Default|GetRestOfLights)
                              (:Output
                                (Variables|Default|SetMult 5e+01)
                                (Utilities|TurnonLights (Variables|Default|GetOtherLights)))))))))))
              (:then_1
                (for _array_element (Utilities|Array|MakeArray (Variables|Default|GetBox) (Variables|Default|GetBox2) (Variables|Default|GetBox3))
                  (Collision|SetCollisionEnabled _array_element "NoCollision"))))))))))

(event EventBeginPlay
  (Variables|Default|SetHasTriggered false)
  (for _array_element (Actor|GetAllChildActors true)
    (bind _asbp_floor_torch (Utilities|Casting|CastToBP_FloorTorch _array_element))
    (Default|SetState _asbp_floor_torch false)))

(fn ConstructionScript
  (bind _returnvalue (Rendering|Material|CreateDynamicMaterialInstance (Variables|Default|GetEyeModel) 0 "/Game/CustomContent/Materials/WallEye/M_EyeOn.M_EyeOn" "None" :!class /Script/Engine.PrimitiveComponent))
  (Variables|Default|SetEyeMat _returnvalue)
  (for _array_element (Actor|GetAllChildActors true)
    (bind _asbp_torch (Utilities|Casting|CastToBP_Torch _array_element)
      (:then
        (Default|SetTorchState _asbp_torch false))
      (:CastFailed
        (bind _asbp_floor_torch (Utilities|Casting|CastToBP_FloorTorch _array_element))
        (Default|SetState _asbp_floor_torch false))))
  (for _array_element_2 (Components|GetChildrenComponents (Variables|Default|GetDefaultSceneRoot) true)
    (bind _aspoint_light_component (Utilities|Casting|CastToPointLightComponent _array_element_2)
      (:then
        (Rendering|Components|Light|SetIntensity _aspoint_light_component 0.0))
      (:CastFailed
        (bind _asrect_light_component (Utilities|Casting|CastToRectLightComponent _array_element_2))
        (Rendering|Components|Light|SetIntensity _asrect_light_component 0.0)))))