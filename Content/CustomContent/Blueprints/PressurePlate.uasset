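; PressurePlate is a puzzle floor plate that shows its pressed or released state by swapping its mesh material.
; SetStartPlate flags it as a start plate with its own material, after which SetPressedState ignores it.
; Pressed-state changes come from outside calls, as the plate's own overlap event is unused.
; When flagged as a target plate, it forwards its state to the parent BasePuzzle actor through SetTorchState.
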(event Custom|SetStartPlate
  (Variables|Default|SetIsStartPlate true)
  (Rendering|Material|SetMaterial (Variables|Default|GetPlateModel) 0 "/Game/CustomContent/Materials/PressurePlate/StartPlate.StartPlate"))

(event Custom|SetPressedState
  (params (Value :type Boolean))
  (if (not (Variables|Default|GetIsStartPlate))
    (Variables|Default|SetIsPressed Value)
    (if Value
      (Rendering|Material|SetMaterial (Variables|Default|GetPlateModel) 0 "/Game/CustomContent/Materials/PressurePlate/PressedPlate.PressedPlate")
      (else
        (Rendering|Material|SetMaterial (Variables|Default|GetPlateModel) 0 "/Game/CustomContent/Materials/PressurePlate/BasePressurePlate.BasePressurePlate")))
    (if (Variables|Default|GetIsTargetPlate)
      (bind _asbase_puzzle (Utilities|Casting|CastToBasePuzzle (Actor|GetAttachParentActor)))
      (Default|SetTorchState _asbase_puzzle Value))))

(event EventBeginPlay)

(event Collision|EventActorBeginOverlap
  (params (OtherActor :type Actor%20Object%20Reference)))

(event EventTick
  (params (DeltaSeconds :type Float%20%28single-precision%29)))

(fn ConstructionScript)