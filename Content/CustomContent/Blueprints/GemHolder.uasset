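; GemHolder is a puzzle pedestal that checks whether enough blue and red gems are placed on it.
; Separate blue and red colliders count gems of matching type, while the pedestal collider tints gems by type and resets them on exit.
; Each count change compares both totals to their requirements, recolours overlapping gems and sets the torch state on the parent BasePuzzle.
; Blue gem recolouring is nested inside the red gem loop.
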(event OnComponentBeginOverlap(PedestalColl)
  (params (OverlappedComponent :type Primitive%20Component%20Object%20Reference) (OtherActor :type Actor%20Object%20Reference) (OtherComp :type Primitive%20Component%20Object%20Reference) (OtherBodyIndex :type Integer) (bFromSweep :type Boolean) (SweepResult :type Hit%20Result%20Structure%20%28by%20ref%29))
  (bind _asgem (Utilities|Casting|CastToGem OtherActor))
  (Default|SetColour _asgem (Variables|/Game/CustomContent/Blueprints/Gem.Gem_C|GetGemType _asgem)))

(event OnComponentEndOverlap(PedestalColl)
  (params (OverlappedComponent :type Primitive%20Component%20Object%20Reference) (OtherActor :type Actor%20Object%20Reference) (OtherComp :type Primitive%20Component%20Object%20Reference) (OtherBodyIndex :type Integer))
  (bind _asgem (Utilities|Casting|CastToGem OtherActor))
  (Default|SetColour _asgem "NewEnumerator0"))

(event OnComponentBeginOverlap(BlueColl)
  (params (OverlappedComponent :type Primitive%20Component%20Object%20Reference) (OtherActor :type Actor%20Object%20Reference) (OtherComp :type Primitive%20Component%20Object%20Reference) (OtherBodyIndex :type Integer) (bFromSweep :type Boolean) (SweepResult :type Hit%20Result%20Structure%20%28by%20ref%29))
  (bind _result (CallFunction|CheckGemType OtherActor "NewEnumerator1"))
  (if _result
    (Variables|Default|SetcurrentBlueGems (+ 1 (Variables|Default|GetcurrentBlueGems)))
    (if (and (>= (Variables|Default|GetcurrentBlueGems) (Variables|Default|GetRequiredBlueGems)) (>= (Variables|Default|GetcurrentRedGems) (Variables|Default|GetRequiredRedGems)))
      (CallFunction|SetCurrentGemColours "NewEnumerator3")
      (CallFunction|SetParentTorchState true)
      (else
        (CallFunction|SetCurrentGemColours "NewEnumerator0")
        (CallFunction|SetParentTorchState false)))))

(event OnComponentEndOverlap(BlueColl)
  (params (OverlappedComponent :type Primitive%20Component%20Object%20Reference) (OtherActor :type Actor%20Object%20Reference) (OtherComp :type Primitive%20Component%20Object%20Reference) (OtherBodyIndex :type Integer))
  (bind _result (CallFunction|CheckGemType OtherActor "NewEnumerator1"))
  (if _result
    (bind _asgem (Utilities|Casting|CastToGem OtherActor))
    (Default|SetColour _asgem "NewEnumerator0")
    (Variables|Default|SetcurrentBlueGems (- (Variables|Default|GetcurrentBlueGems) 1))
    (if (and (>= (Variables|Default|GetcurrentBlueGems) (Variables|Default|GetRequiredBlueGems)) (>= (Variables|Default|GetcurrentRedGems) (Variables|Default|GetRequiredRedGems)))
      (CallFunction|SetCurrentGemColours "NewEnumerator3")
      (CallFunction|SetParentTorchState true)
      (else
        (CallFunction|SetCurrentGemColours "NewEnumerator0")
        (CallFunction|SetParentTorchState false)))))

(event OnComponentBeginOverlap(RedColl)
  (params (OverlappedComponent :type Primitive%20Component%20Object%20Reference) (OtherActor :type Actor%20Object%20Reference) (OtherComp :type Primitive%20Component%20Object%20Reference) (OtherBodyIndex :type Integer) (bFromSweep :type Boolean) (SweepResult :type Hit%20Result%20Structure%20%28by%20ref%29))
  (bind _result (CallFunction|CheckGemType OtherActor "NewEnumerator2"))
  (if _result
    (Variables|Default|SetcurrentRedGems (+ 1 (Variables|Default|GetcurrentRedGems)))
    (if (and (>= (Variables|Default|GetcurrentBlueGems) (Variables|Default|GetRequiredBlueGems)) (>= (Variables|Default|GetcurrentRedGems) (Variables|Default|GetRequiredRedGems)))
      (CallFunction|SetCurrentGemColours "NewEnumerator3")
      (CallFunction|SetParentTorchState true)
      (else
        (CallFunction|SetCurrentGemColours "NewEnumerator0")
        (CallFunction|SetParentTorchState false)))))

(event OnComponentEndOverlap(RedColl)
  (params (OverlappedComponent :type Primitive%20Component%20Object%20Reference) (OtherActor :type Actor%20Object%20Reference) (OtherComp :type Primitive%20Component%20Object%20Reference) (OtherBodyIndex :type Integer))
  (bind _result (CallFunction|CheckGemType OtherActor "NewEnumerator2"))
  (if _result
    (bind _asgem (Utilities|Casting|CastToGem OtherActor))
    (Default|SetColour _asgem "NewEnumerator0")
    (Variables|Default|SetcurrentRedGems (- (Variables|Default|GetcurrentRedGems) 1))
    (if (and (>= (Variables|Default|GetcurrentBlueGems) (Variables|Default|GetRequiredBlueGems)) (>= (Variables|Default|GetcurrentRedGems) (Variables|Default|GetRequiredRedGems)))
      (CallFunction|SetCurrentGemColours "NewEnumerator3")
      (CallFunction|SetParentTorchState true)
      (else
        (CallFunction|SetCurrentGemColours "NewEnumerator0")
        (CallFunction|SetParentTorchState false)))))

(event EventBeginPlay)

(event Collision|EventActorBeginOverlap
  (params (OtherActor :type Actor%20Object%20Reference)))

(event EventTick
  (params (DeltaSeconds :type Float%20%28single-precision%29)))

(fn ConstructionScript)

(fn CheckGemType
  (params (Object :type Object%20Object%20Reference) (DesiredType :type GemColours%20Enum :default "NewEnumerator0"))
  (bind _asgem (Utilities|Casting|CastToGem Object))
  (return (== (Variables|/Game/CustomContent/Blueprints/Gem.Gem_C|GetGemType _asgem) (Math|Byte|MakeLiteralByte DesiredType))))

(fn SetCurrentGemColours
  (params (ColourToSet :type GemColours%20Enum :default "NewEnumerator0"))
  (for _array_element (Collision|GetOverlappingActors (Variables|Default|GetRedColl) "/Game/CustomContent/Blueprints/Gem.Gem_C" :!class /Script/Engine.PrimitiveComponent)
    (bind _asgem (Utilities|Casting|CastToGem _array_element))
    (Default|SetColour _asgem ColourToSet)
    (for _array_element_2 (Collision|GetOverlappingActors (Variables|Default|GetBlueColl) "/Game/CustomContent/Blueprints/Gem.Gem_C" :!class /Script/Engine.PrimitiveComponent)
      (bind _asgem_2 (Utilities|Casting|CastToGem _array_element_2))
      (Default|SetColour _asgem_2 ColourToSet))))

(fn SetParentTorchState
  (params (Value :type Boolean))
  (bind _asbase_puzzle (Utilities|Casting|CastToBasePuzzle (Actor|GetAttachParentActor)))
  (Default|SetTorchState _asbase_puzzle Value))