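; BP_RiddlePuzzle is a pressure plate puzzle where a randomized riddle about a walking totem points to the target plate.
; On BeginPlay it spawns and attaches a square grid of plates, marking the centre as the start.
; It rolls in-bounds north, east, south and west moves from the centre, nudging north if they end there, and flags the resulting plate as target.
; SetRiddleText writes those step counts onto the east and west wall texts.
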(event Custom|SetRiddleText
  ;[0.15 0.15 0.15 0.5] Create riddle text using generated move numbers
  ;[0.15 0.15 0.15 0.5] Set text on wall
  (Rendering|Components|TextRender|SetText (Variables|Default|GetEast%20Wall%20Text) (Utilities|Text|ToText(String) (Utilities|String|Append (Utilities|String|Append (Utilities|String|Append (Utilities|String|Append "The totem awoke in a strange land.<br>It walked " (Utilities|String|ToString(Integer) (Variables|Default|GetnorthMove))) " steps North and ") (Utilities|String|ToString(Integer) (Variables|Default|GeteastMove))) " steps East before stopping.")))
  (Rendering|Components|TextRender|SetText (Variables|Default|GetWest%20Wall%20Text) (Utilities|Text|ToText(String) (Utilities|String|Append (Utilities|String|Append (Utilities|String|Append (Utilities|String|Append "Then it turned, and walked " (Utilities|String|ToString(Integer) (Variables|Default|GetsouthMove))) " steps South<br>and ") (Utilities|String|ToString(Integer) (Variables|Default|GetwestMove))) " steps West... and it rested."))))

(event EventBeginPlay
  (bind _returnvalue (Utilities|GetMiddleIndex))
  (bind _rowlengthwidth (Variables|Default|GetRowLengthWidth))
  (bind _startpressurespawn (Variables|Default|GetStartPressureSpawn))
  (bind _returnvalue_2 (Transformation|GetWorldLocation _startpressurespawn))
  (bind _returnvalue_3 (- _rowlengthwidth 1))
  (bind (_x _y _z) (Math|Vector|BreakVector _returnvalue_2))
  ;[0.15 0.15 0.15 0.5] Loop for row and column of plates to spawn
  (for _index (range 0 _returnvalue_3)
    (for _index_2 (range 0 _returnvalue_3)
      ;[0.15 0.15 0.15 0.5] Spawn plate at calculated position
      (bind _returnvalue_4 (Game|SpawnActorfromClass "/Game/CustomContent/Blueprints/PressurePlate.PressurePlate_C" (Math|Transform|MakeTransform (Math|Vector|MakeVector (+ _x (* _index -1e+02)) (+ (* _index_2 -1e+02) _y) _z)) "Undefined" "MultiplyWithRoot" 0 0))
      ;[0.15 0.15 0.15 0.5] Make plate a child of this blueprint
      (Transformation|AttachActorToActor _returnvalue_4 self "None" "KeepWorld" "KeepWorld" "KeepWorld" true)
      ;[0.15 0.15 0.15 0.5] Add spawned plate to list
      (Utilities|Array|Add (Variables|Default|GetLocalPlateArray) _returnvalue_4)
      ;[0.15 0.15 0.15 0.5] If spawned plate is in the centre, set as start plate
      (if (and (== _index _returnvalue) (== _index_2 _returnvalue))
        (Default|SetStartPlate _returnvalue_4))))
  ;[0.15 0.15 0.15 0.5] Set starting X and Y pos to centre
  (bind _output_get (Variables|Default|SetxIndex (Utilities|GetMiddleIndex)))
  (Variables|Default|SetyIndex _output_get)
  ;[0.15 0.15 0.15 0.5] Get north move within range
  (bind _output_get_2 (Variables|Default|SetnorthMove (Math|Random|RandomIntegerinRange 1 (- (Utilities|GetAdjustedRowLengthWidth) (Variables|Default|GetyIndex)))))
  (Variables|Default|SetyIndex (+ (Variables|Default|GetyIndex) _output_get_2))
  ;[0.15 0.15 0.15 0.5] Get east move within range
  (bind _output_get_3 (Variables|Default|SeteastMove (Math|Random|RandomIntegerinRange 1 (- (Utilities|GetAdjustedRowLengthWidth) (Variables|Default|GetxIndex)))))
  (Variables|Default|SetxIndex (+ (Variables|Default|GetxIndex) _output_get_3))
  ;[0.15 0.15 0.15 0.5] Get south move within range
  (bind _output_get_4 (Variables|Default|SetsouthMove (Math|Random|RandomIntegerinRange 1 (Variables|Default|GetyIndex))))
  (Variables|Default|SetyIndex (- (Variables|Default|GetyIndex) _output_get_4))
  ;[0.15 0.15 0.15 0.5] Get west move within range
  (bind _output_get_5 (Variables|Default|SetwestMove (Math|Random|RandomIntegerinRange 1 (Variables|Default|GetxIndex))))
  (Variables|Default|SetxIndex (- (Variables|Default|GetxIndex) _output_get_5))
  ;[0.15 0.15 0.15 0.5] If the target plate is in the centre, move it up by one
  (if (and (== (Variables|Default|GetxIndex) (Utilities|GetMiddleIndex)) (== (Variables|Default|GetyIndex) (Utilities|GetMiddleIndex)))
    (Variables|Default|SetyIndex (+ (Variables|Default|GetyIndex) 1))
    (Variables|Default|SetnorthMove (+ (Variables|Default|GetnorthMove) 1)))
  ;[0.15 0.15 0.15 0.5] Find the target plate and set it to be target
  (Variables|/Game/CustomContent/Blueprints/PressurePlate.PressurePlate_C|SetIsTargetPlate (Utilities|Get2DArrayValue (Variables|Default|GetxIndex) (Variables|Default|GetyIndex)) true)
  (CallFunction|SetRiddleText)
  (|CallParentFunction))

(event Collision|EventActorBeginOverlap
  (params (OtherActor :type Actor%20Object%20Reference))
  (|CallParentFunction OtherActor) ; This node is disabled and will not be called.\nDrag off pins to build functionality.
)

(event EventTick
  (params (DeltaSeconds :type Float%20%28single-precision%29))
  (|CallParentFunction DeltaSeconds) ; This node is disabled and will not be called.\nDrag off pins to build functionality.
)

(fn ConstructionScript
  (|CallParentFunction))