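; Riddle puzzle actor that spawns a square grid of pressure plates and hides a target plate for a randomized text clue.
; On BeginPlay it marks the center plate as start, then rolls bounded North, East, South and West moves, nudging a (0,0) result one step North.
; The end cell, looked up in the flat plate array, becomes the target, and the step counts form a totem story on two wall texts.
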(event Custom|SetRiddleText
  (Rendering|Components|TextRender|SetText (Variables|Default|GetEast%20Wall%20Text) (Utilities|Text|ToText(String) (Utilities|String|Append (Utilities|String|Append (Utilities|String|Append (Utilities|String|Append "The totem awoke in a strange land.<br>It walked " (Utilities|String|ToString(Integer) (Variables|Default|GetnorthMove))) " steps North and ") (Utilities|String|ToString(Integer) (Variables|Default|GeteastMove))) " steps East before stopping.")))
  (Rendering|Components|TextRender|SetText (Variables|Default|GetWest%20Wall%20Text) (Utilities|Text|ToText(String) (Utilities|String|Append (Utilities|String|Append (Utilities|String|Append (Utilities|String|Append "Then it turned, and walked " (Utilities|String|ToString(Integer) (Variables|Default|GetsouthMove))) " steps South<br>and ") (Utilities|String|ToString(Integer) (Variables|Default|GetwestMove))) " steps West... and it rested."))))

(event EventBeginPlay
  (bind _returnvalue (Utilities|GetMiddleIndex))
  (bind _rowlengthwidth (Variables|Default|GetRowLengthWidth))
  (bind _startpressurespawn (Variables|Default|GetStartPressureSpawn))
  (bind _returnvalue_2 (Transformation|GetWorldLocation _startpressurespawn))
  (bind _returnvalue_3 (- _rowlengthwidth 1))
  (bind (_x _y _z) (Math|Vector|BreakVector _returnvalue_2))
  ;[0.15 0.15 0.15 0.5] Place Plates
  (for _index (range 0 _returnvalue_3)
    (for _index_2 (range 0 _returnvalue_3)
      (bind _returnvalue_4 (Game|SpawnActorfromClass "/Game/CustomContent/Blueprints/PressurePlate.PressurePlate_C" (Math|Transform|MakeTransform (Math|Vector|MakeVector (+ _x (* _index -1e+02)) (+ _y (* _index_2 -1e+02)) _z)) "Undefined" "MultiplyWithRoot" 0 0))
      (Utilities|Array|Add (Variables|Default|GetLocalPlateArray) _returnvalue_4)
      (if (and (== _index_2 _returnvalue) (== _index _returnvalue))
        (Default|SetStartPlate _returnvalue_4))))
  (bind _output_get (Variables|Default|SetxIndex (Utilities|GetMiddleIndex)))
  (Variables|Default|SetyIndex _output_get)
  (bind _output_get_2 (Variables|Default|SetnorthMove (Math|Random|RandomIntegerinRange 1 (- (Utilities|GetAdjustedRowLengthWidth) (Variables|Default|GetyIndex)))))
  (Variables|Default|SetyIndex (+ (Variables|Default|GetyIndex) _output_get_2))
  (bind _output_get_3 (Variables|Default|SeteastMove (Math|Random|RandomIntegerinRange 1 (- (Utilities|GetAdjustedRowLengthWidth) (Variables|Default|GetxIndex)))))
  (Variables|Default|SetxIndex (+ (Variables|Default|GetxIndex) _output_get_3))
  (bind _output_get_4 (Variables|Default|SetsouthMove (Math|Random|RandomIntegerinRange 1 (Variables|Default|GetyIndex))))
  (Variables|Default|SetyIndex (- (Variables|Default|GetyIndex) _output_get_4))
  (bind _output_get_5 (Variables|Default|SetwestMove (Math|Random|RandomIntegerinRange 1 (Variables|Default|GetxIndex))))
  (Variables|Default|SetxIndex (- (Variables|Default|GetxIndex) _output_get_5))
  (if (and (== (Variables|Default|GetxIndex) 0) (== (Variables|Default|GetyIndex) 0))
    (Variables|Default|SetyIndex (+ (Variables|Default|GetyIndex) 1))
    (Variables|Default|SetnorthMove (+ (Variables|Default|GetnorthMove) 1)))
  (Variables|/Game/CustomContent/Blueprints/PressurePlate.PressurePlate_C|SetIsTargetPlate (Utilities|Get2DArrayValue (Variables|Default|GetxIndex) (Variables|Default|GetyIndex)) true)
  (CallFunction|SetRiddleText)
  (|CallParentFunction))

(event Collision|EventActorBeginOverlap
  (params (OtherActor :type Actor%20Object%20Reference))
  (|CallParentFunction OtherActor) ; This node is disabled and will not be called.\nDrag off pins to build functionality.
)

(event EventTick
  (params (DeltaSeconds :type Float%20%28single-precision%29))
  (|CallParentFunction DeltaSeconds) ; This node is disabled and will not be called.\nDrag off pins to build functionality.
)

(fn ConstructionScript
  (|CallParentFunction))