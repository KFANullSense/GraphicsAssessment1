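; Gem sorting puzzle that randomizes the number, placement and color mix of gems on BeginPlay.
; It shuffles all placed BP_GemSpawn actors and keeps roughly half to three quarters of them.
; A random blue/red split, intended to include both colors, sets the required counts on its child-actor BP_GemHolder.
; It then spawns a BP_Gem at each chosen point, typed by index, calling parent BeginPlay inside that loop.
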(event EventBeginPlay
  (bind _outactors (Actor|GetAllActorsOfClass "/Game/CustomContent/Blueprints/SpawnPoints/BP_GemSpawn.BP_GemSpawn_C"))
  ;[0.15 0.15 0.15 0.5] Get a random collection of gem spawn points, between 50% and 75% of the whole set
  (Utilities|Array|Shuffle _outactors) ; Randomize order of gem spawns
  (Utilities|Array|Resize _outactors (Math|Random|RandomIntegerinRange (Math|Float|Round (* (Math|Conversions|ToFloat(Integer) (Utilities|Array|Length _outactors)) 0.5)) (Math|Float|Round (* (Math|Conversions|ToFloat(Integer) (Utilities|Array|Length _outactors)) 0.75))))
  ;[0.15 0.15 0.15 0.5] Get random number of gems to be blue
  (bind _asbp_gem_holder (Utilities|Casting|CastToBP_GemHolder (Variables|/Script/Engine.ChildActorComponent|GetChildActor (Variables|Default|GetGemHolder))))
  (bind _output_get (Variables|Default|SetRandomResizeValue (Math|Random|RandomIntegerinRange 1 (- (Utilities|Array|Length _outactors) 1))))
  (Variables|/Game/CustomContent/Blueprints/BP_GemHolder.BP_GemHolder_C|SetRequiredBlueGems _asbp_gem_holder _output_get)
  ;[0.15 0.15 0.15 0.5] Set the remaining gems to be red
  (Variables|/Game/CustomContent/Blueprints/BP_GemHolder.BP_GemHolder_C|SetRequiredRedGems _asbp_gem_holder (- (Utilities|Array|Length _outactors) _output_get))
  ;[0.15 0.15 0.15 0.5] For each valid spawn point, spawn a gem
  (for (_array_element _array_index) _outactors
    (bind _returnvalue (Game|SpawnActorfromClass "/Game/CustomContent/Blueprints/BP_Gem.BP_Gem_C" (Transformation|GetWorldTransform (Variables|/Game/CustomContent/Blueprints/SpawnPoints/BP_GemSpawn.BP_GemSpawn_C|GetDefaultSceneRoot _array_element)) "Undefined" "MultiplyWithRoot" 0 0))
    ;[0.15 0.15 0.15 0.5] For each gem, set if it is red or blue based on the index
    (if (< _array_index _output_get)
      (Variables|/Game/CustomContent/Blueprints/BP_Gem.BP_Gem_C|SetGemType _returnvalue "NewEnumerator1")
      (else
        (Variables|/Game/CustomContent/Blueprints/BP_Gem.BP_Gem_C|SetGemType _returnvalue "NewEnumerator2")))
    (|CallParentFunction)))

(event Collision|EventActorBeginOverlap
  (params (OtherActor :type Actor%20Object%20Reference))
  (|CallParentFunction OtherActor) ; This node is disabled and will not be called.\nDrag off pins to build functionality.
)

(event EventTick
  (params (DeltaSeconds :type Float%20%28single-precision%29))
  (|CallParentFunction DeltaSeconds) ; This node is disabled and will not be called.\nDrag off pins to build functionality.
)

(fn ConstructionScript
  (|CallParentFunction))