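; First-person character Blueprint that lets the player pick up, carry and drop HoldableObject actors with the left mouse button.
; A click line-traces on Visibility from the camera out to GrabRange and grabs a valid hit component with the PhysicsHandle, while the next click releases it.
; While holding, Tick moves the handle target to the same camera-forward point computed by GetGrabRaycast.
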(event EventBeginPlay)

(event Collision|EventActorBeginOverlap
  (params (OtherActor :type Actor%20Object%20Reference)))

(event EventTick
  (params (DeltaSeconds :type Float%20%28single-precision%29))
  (if (Variables|Default|GetisHoldingObject)
    (bind _returnvector (CallFunction|GetGrabRaycast (Variables|Default|GetGrabRange)))
    (Physics|Components|PhysicsHandle|SetTargetLocation (Variables|Default|GetPhysicsHandle) _returnvector)))

(event Input|MouseEvents|LeftMouseButton
  (params (Key :type Key%20Structure :default "None"))
  (:Pressed
    (if (Variables|Default|GetisHoldingObject)
      (if (Variables|Default|GetisHoldingObject)
        (Physics|Components|PhysicsHandle|ReleaseComponent (Variables|Default|GetPhysicsHandle))
        (Variables|Default|SetisHoldingObject false))
      (else
        (bind _returnvector (CallFunction|GetGrabRaycast (Variables|Default|GetGrabRange)))
        (bind (_outhit _returnvalue) (Collision|LineTraceByChannel (Transformation|GetWorldLocation (Variables|Default|GetFirstPersonCamera)) _returnvector "TraceTypeQuery1" false 0 "None"))
        (if _returnvalue
          (if (Utilities|ClassIsChildOf (Utilities|GetClass (Components|GetOwner (.HitComponent (Collision|BreakHitResult _outhit)))) "/Game/CustomContent/Blueprints/HoldableObject.HoldableObject_C")
            (Physics|Components|PhysicsHandle|GrabComponentatLocationwithRotation (Variables|Default|GetPhysicsHandle) (.HitComponent (Collision|BreakHitResult _outhit)) "None" (Transformation|GetWorldLocation (.HitComponent (Collision|BreakHitResult _outhit))) "0, 0, 0")
            (Variables|Default|SetisHoldingObject true)))))))

(fn ConstructionScript
  (|CallParentFunction))

(fn GetGrabRaycast
  (params (GrabRange :type Float%20%28double-precision%29))
  (bind _firstpersoncamera (Variables|Default|GetFirstPersonCamera))
  (return (+ (Transformation|GetWorldLocation _firstpersoncamera) (* (Math|Vector|GetForwardVector (Transformation|GetWorldRotation _firstpersoncamera)) GrabRange))))