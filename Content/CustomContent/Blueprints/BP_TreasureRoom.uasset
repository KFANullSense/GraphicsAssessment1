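; BP_TreasureRoom is a puzzle room whose door opens once every torch in the level is lit.
; On BeginPlay it caches all BP_Torch actors, then checks them whenever the player enters the door trigger while the door is closed.
; A separate trigger opens the treasure chest on the player's first overlap.
; Both openings play animations on door and chest Child Actors.
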(event OnComponentBeginOverlap(DoorColl)
  (params (OverlappedComponent :type Primitive%20Component%20Object%20Reference) (OtherActor :type Actor%20Object%20Reference) (OtherComp :type Primitive%20Component%20Object%20Reference) (OtherBodyIndex :type Integer) (bFromSweep :type Boolean) (SweepResult :type Hit%20Result%20Structure%20%28by%20ref%29))
  ;[0.15 0.15 0.15 0.5] If player walks in door room and it's not open, continue
  (Utilities|Casting|CastToBP_CustomFPSCharacter OtherActor)
  (if (not (Variables|Default|GetIsDoorOpen))
    (Variables|Default|SetAllTorchesLit true) ; Set all torches lit at the start, set to false if any are not lit
    ;[0.15 0.15 0.15 0.5] Iterate through torches, if any aren't lit break the loop
    (bind _array_element (Utilities|Array|ForEachLoopwithBreak (Variables|Default|GetTorches) :!label _label)
      (:LoopBody
        (if (not (Variables|/Game/CustomContent/Blueprints/BP_Torch.BP_Torch_C|GetIsTorchLit _array_element))
          (Variables|Default|SetAllTorchesLit false)
          (goto _label Break)))
      (:Completed
        ;[0.15 0.15 0.15 0.5] If all torches are lit at the end, open the door
        (if (Variables|Default|GetAllTorchesLit)
          (CallFunction|OpenDoor))))))

(event OnComponentBeginOverlap(TreasureColl)
  (params (OverlappedComponent :type Primitive%20Component%20Object%20Reference) (OtherActor :type Actor%20Object%20Reference) (OtherComp :type Primitive%20Component%20Object%20Reference) (OtherBodyIndex :type Integer) (bFromSweep :type Boolean) (SweepResult :type Hit%20Result%20Structure%20%28by%20ref%29))
  ;[0.15 0.15 0.15 0.5] If player walks close to chest, open it
  (Utilities|Casting|CastToBP_CustomFPSCharacter OtherActor)
  (if (not (Variables|Default|GetIsChestOpen))
    (Variables|Default|SetIsChestOpen true)
    (CallFunction|OpenChest)))

(event Custom|OpenDoor
  (Variables|Default|SetIsDoorOpen true)
  (bind _asbp_treasure_door (Utilities|Casting|CastToBP_TreasureDoor (Variables|/Script/Engine.ChildActorComponent|GetChildActor (Variables|Default|GetTreasureDoor))))
  (Default|OpenDoorAnimation _asbp_treasure_door))

(event Custom|OpenChest
  (bind _asbp_treasure_chest (Utilities|Casting|CastToBP_TreasureChest (Variables|/Script/Engine.ChildActorComponent|GetChildActor (Variables|Default|GetTreasureChest))))
  (Default|OpenChestAnimation _asbp_treasure_chest))

(event EventBeginPlay
  ;[0.15 0.15 0.15 0.5] On start, get all torches and store them for later reference
  (bind _outactors (Actor|GetAllActorsOfClass "/Game/CustomContent/Blueprints/BP_Torch.BP_Torch_C"))
  (Variables|Default|SetTorches _outactors))

(event Collision|EventActorBeginOverlap
  (params (OtherActor :type Actor%20Object%20Reference)))

(fn ConstructionScript)