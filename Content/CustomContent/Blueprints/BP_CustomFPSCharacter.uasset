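; First-person player character that picks up, carries and drops BP_HoldableObject actors and turns math-puzzle spin wheels with left click.
; A camera line trace within GrabRange finds the target, which a PhysicsHandle grabs; a second click zeroes its velocity and releases it.
; Each tick the held object follows the point ahead of the camera, yawed to face it using its StartingZRot offset.
; With empty hands, clicking components tagged LWheel or RWheel increments that BP_SpinWheel side.
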(event EventBeginPlay)

(event Collision|EventActorBeginOverlap
  (params (OtherActor :type Actor%20Object%20Reference)))

(event EventTick
  (params (DeltaSeconds :type Float%20%28single-precision%29))
  (bind _physicshandle (Variables|Default|GetPhysicsHandle))
  (bind _returnvalue (Class|PhysicsHandleComponent|GetGrabbedComponent _physicshandle))
  ;[0.15 0.15 0.15 0.5] Move held object to target position every frame
  (if (Variables|Default|GetisHoldingObject)
    (bind _returnvector (CallFunction|GetGrabRaycast (Variables|Default|GetGrabRange)))
    (Physics|Components|PhysicsHandle|SetTargetLocation _physicshandle _returnvector)
    ;;[0.15 0.15 0.15 0.5] Rotate held object to face camera
    (bind _asbp_holdable_object (Utilities|Casting|CastToBP_HoldableObject (Components|GetOwner _returnvalue)))
    (bind _rotationvalue (CallFunction|GetRotationtoCamera _asbp_holdable_object))
    (Transformation|SetRelativeRotation _returnvalue _rotationvalue false false)))

(event Input|MouseEvents|LeftMouseButton
  (params (Key :type Key%20Structure :default "None"))
  ;[0.15 0.15 0.15 0.5] If not holding an object, can click on spinwheel (for Math puzzle)
  (:Pressed
    (if (not (Variables|Default|GetisHoldingObject))
      (bind _returnvector (CallFunction|GetGrabRaycast (Variables|Default|GetGrabRange)))
      (bind (_outhit _returnvalue) (Collision|LineTraceByChannel (Transformation|GetWorldLocation (Variables|Default|GetFirstPersonCamera)) _returnvector "TraceTypeQuery1" false 0 "None"))
      (if _returnvalue
        (if (Components|ComponentHasTag (.HitComponent (Collision|BreakHitResult _outhit)) "LWheel")
          (bind _asbp_spin_wheel (Utilities|Casting|CastToBP_SpinWheel (.HitActor (Collision|BreakHitResult _outhit))))
          (Default|IncrementLeftWheel _asbp_spin_wheel)
          (elif (Components|ComponentHasTag (.HitComponent (Collision|BreakHitResult _outhit)) "RWheel")
            (bind _asbp_spin_wheel_2 (Utilities|Casting|CastToBP_SpinWheel (.HitActor (Collision|BreakHitResult _outhit))))
            (Default|IncrementRightWheel _asbp_spin_wheel_2)))))))

(event Input|MouseEvents|LeftMouseButton
  (params (Key :type Key%20Structure :default "None"))
  (bind _physicshandle (Variables|Default|GetPhysicsHandle))
  (bind _returnvalue (Class|PhysicsHandleComponent|GetGrabbedComponent _physicshandle))
  ;[0.15 0.15 0.15 0.5] Pick up and drop object on Left Click
  (:Pressed
    (if (Variables|Default|GetisHoldingObject)
      ;;[0.15 0.15 0.15 0.5] If object held, reset velocity and drop it
      (Physics|SetPhysicsLinearVelocity _returnvalue "0, 0, 0" false "None")
      (Class|PrimitiveComponent|SetPhysicsAngularVelocityinDegrees _returnvalue "0, 0, 0" false "None")
      (Physics|Components|PhysicsHandle|ReleaseComponent _physicshandle)
      (Variables|Default|SetisHoldingObject false)
      (else
        ;;[0.15 0.15 0.15 0.5] Check for holdable object where player is clicking
        (bind _returnvector (CallFunction|GetGrabRaycast (Variables|Default|GetGrabRange)))
        (bind (_outhit _returnvalue_2) (Collision|LineTraceByChannel (Transformation|GetWorldLocation (Variables|Default|GetFirstPersonCamera)) _returnvector "TraceTypeQuery1" false 0 "None"))
        (if _returnvalue_2
          ;;[0.15 0.15 0.15 0.5] Make sure clicked object's base class is holdable object
          (if (Utilities|ClassIsChildOf (Utilities|GetClass (Components|GetOwner (.HitComponent (Collision|BreakHitResult _outhit)))) "/Game/CustomContent/Blueprints/BP_HoldableObject.BP_HoldableObject_C")
            (bind _asbp_holdable_object (Utilities|Casting|CastToBP_HoldableObject (.HitActor (Collision|BreakHitResult _outhit))))
            ;;[0.15 0.15 0.15 0.5] Turn object to face camera and pick up
            (bind _rotationvalue (CallFunction|GetRotationtoCamera _asbp_holdable_object))
            (Transformation|SetRelativeRotation (.HitComponent (Collision|BreakHitResult _outhit)) _rotationvalue false false)
            (Class|PhysicsHandleComponent|GrabComponentatLocation (Variables|Default|GetPhysicsHandle) (.HitComponent (Collision|BreakHitResult _outhit)) "None" (Transformation|GetWorldLocation (.HitComponent (Collision|BreakHitResult _outhit))))
            (Variables|Default|SetisHoldingObject true)))))))

(fn ConstructionScript
  (|CallParentFunction))

(fn GetGrabRaycast
  (params (GrabRange :type Float%20%28double-precision%29))
  (bind _firstpersoncamera (Variables|Default|GetFirstPersonCamera))
  (return (+ (Transformation|GetWorldLocation _firstpersoncamera) (* (Math|Vector|GetForwardVector (Transformation|GetWorldRotation _firstpersoncamera)) GrabRange))))

(fn GetRotationtoCamera
  (params (ObjToRotate :type BP%20Holdable%20Object%20Object%20Reference))
  (return (Math|Rotator|MakeRotator 0.0 0.0 (- (.Yaw (Math|Rotator|BreakRotator (Transformation|GetWorldRotation (Variables|Default|GetFirstPersonCamera)))) (Variables|/Game/CustomContent/Blueprints/BP_HoldableObject.BP_HoldableObject_C|GetStartingZRot ObjToRotate)))))