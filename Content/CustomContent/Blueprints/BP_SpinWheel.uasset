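; BP_SpinWheel is a two-wheel number dial puzzle whose answer is (A+B)*(C-D), randomized on BeginPlay.
; It writes the four variable values onto four randomly chosen BP_EquationSpawn actors.
; Increment events advance a wheel's digit with wraparound and rotate it by timeline, ignoring input mid-spin.
; During rotation, it compares the two-digit value to the answer and sets the parent BP_BasePuzzle's torch state.
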(event Custom|IncrementLeftWheel
  (bind _wheell (Variables|Default|GetWheelL))
  ;[0.15 0.15 0.15 0.5] If wheel isn't rotating, increment then rotate
  (if (not (Variables|Default|GetLRotating))
    (bind _output (CallFunction|IncrementNum (Variables|Default|GetLeftWheelVal)))
    (Variables|Default|SetLeftWheelVal _output)
    (Variables|Default|SetLRotating true)
    (Variables|Default|SetStartLRot (Variables|/Script/Engine.SceneComponent|GetRelativeRotation _wheell))
    ;[0.15 0.15 0.15 0.5] Rotate wheel over time
    (bind _timepassed (Timeline|LWheelTimeline PlayFromStart)
      (:Update
        (Transformation|SetRelativeRotation _wheell (Math|Rotator|CombineRotators (Math|Rotator|MakeRotator (* _timepassed -36.0) 0.0 0.0) (Variables|Default|GetStartLRot)) false false)
        ;[0.15 0.15 0.15 0.5] After rotation, validate number and set torch state
        (bind _result (CallFunction|ValidateWheelNum))
        (bind _asbp_base_puzzle (Utilities|Casting|CastToBP_BasePuzzle (Actor|GetAttachParentActor)))
        (Default|SetTorchState _asbp_base_puzzle _result))
      (:Finished
        (Variables|Default|SetLRotating false)))))

(event Custom|IncrementRightWheel
  (bind _wheelr (Variables|Default|GetWheelR))
  ;[0.15 0.15 0.15 0.5] Same as above but for left wheel
  (if (not (Variables|Default|GetRRotating))
    (bind _output (CallFunction|IncrementNum (Variables|Default|GetRightWheelVal)))
    (Variables|Default|SetRightWheelVal _output)
    (Variables|Default|SetRRotating true)
    (Variables|Default|SetStartRRot (Variables|/Script/Engine.SceneComponent|GetRelativeRotation _wheelr))
    ;[0.15 0.15 0.15 0.5] Same as above
    (bind _timepassed (Timeline|RWheelTimeline PlayFromStart)
      (:Update
        (Transformation|SetRelativeRotation _wheelr (Math|Rotator|CombineRotators (Variables|Default|GetStartRRot) (Math|Rotator|MakeRotator (* _timepassed -36.0) 0.0 0.0)) false false)
        ;[0.15 0.15 0.15 0.5] After rotation, validate number and set torch state
        (bind _result (CallFunction|ValidateWheelNum))
        (bind _asbp_base_puzzle (Utilities|Casting|CastToBP_BasePuzzle (Actor|GetAttachParentActor)))
        (Default|SetTorchState _asbp_base_puzzle _result))
      (:Finished
        (Variables|Default|SetRRotating false)))))

(event EventBeginPlay
  ;[0.15 0.15 0.15 0.5] Assign D variable between 1 and 9, and C variable within 5 above it (clamp between 1-10)
  (bind _output_get (Variables|Default|SetdVar (Math|Random|RandomIntegerinRange 1 9)))
  (Variables|Default|SetcVar (Math|Integer|Clamp(Integer) (Math|Random|RandomIntegerinRange (+ _output_get 1) (+ _output_get 5)) 1 10))
  ;[0.15 0.15 0.15 0.5] Set A and B to be between 1-9
  (Variables|Default|SetbVar (Math|Random|RandomIntegerinRange 1 9))
  (Variables|Default|SetaVar (Math|Random|RandomIntegerinRange 1 9))
  ;[0.15 0.15 0.15 0.5] Calculate solution
  (Variables|Default|SetTargetNumber (* (+ (Variables|Default|GetaVar) (Variables|Default|GetbVar)) (- (Variables|Default|GetcVar) (Variables|Default|GetdVar))))
  ;[0.15 0.15 0.15 0.5] Pick four random spots to write the equation text
  (bind _outactors (Actor|GetAllActorsOfClass "/Game/CustomContent/Blueprints/SpawnPoints/BP_EquationSpawn.BP_EquationSpawn_C"))
  (Utilities|Array|Shuffle _outactors)
  (Utilities|Array|Resize _outactors 4)
  (Utilities|FlowControl|Sequence
    (:then_0
      ;[0.15 0.15 0.15 0.5] Set wall text to variable numbers
      (Default|SetText (Utilities|Array|Get(acopy) _outactors) (Utilities|String|Append "A = " (Utilities|String|ToString(Integer) (Variables|Default|GetaVar)))))
    (:then_1
      (Default|SetText (Utilities|Array|Get(acopy) _outactors 1) (Utilities|String|Append "B = " (Utilities|String|ToString(Integer) (Variables|Default|GetbVar)))))
    (:then_2
      (Default|SetText (Utilities|Array|Get(acopy) _outactors 2) (Utilities|String|Append "C = " (Utilities|String|ToString(Integer) (Variables|Default|GetcVar)))))
    (:then_3
      (Default|SetText (Utilities|Array|Get(acopy) _outactors 3) (Utilities|String|Append "D = " (Utilities|String|ToString(Integer) (Variables|Default|GetdVar)))))))

(fn ConstructionScript)

(fn CalculateWheelVal
  (return (+ (* (Variables|Default|GetLeftWheelVal) 10) (Variables|Default|GetRightWheelVal))))

(fn ValidateWheelNum
  (bind _finalnum (CallFunction|CalculateWheelVal))
  (return (== _finalnum (Variables|Default|GetTargetNumber))))

(fn IncrementNum
  (params (Input :type Integer))
  (bind _returnvalue (+ Input 1))
  ;[0.15 0.15 0.15 0.5] If number goes to 10, reset to 0
  (if (>= _returnvalue 10)
    (return (- _returnvalue 10))
    (else
      (return _returnvalue))))